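; Collectable pickup actor that spins and bobs in the level until the player collects it.
; When the player pawn overlaps it, it plays a coin sound, spawns a particle effect at its Sphere component and destroys itself.
; Tick adds a fixed per-frame local rotation and calls Play on the Bob timeline, whose track is applied as an additive local offset without sweep.
; It updates no score or inventory.
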(event EventBeginPlay)

(event Collision|EventActorBeginOverlap
  (params (OtherActor :type Actor%20Object%20Reference))
  (if (== OtherActor (Game|Player|GetPlayerPawn 0))
    (Audio|PlaySound2D "/Game/SoundEffects/Pickup_Coin31.Pickup_Coin31" 1.0 1.0 0.0 0 0)
    (Effects|SpawnEmitteratLocation "/Game/Particles/p_collectable.p_collectable" (Transformation|GetWorldLocation (Variables|Default|GetSphere)))
    (Actor|DestroyActor)))

(event EventTick
  (params (DeltaSeconds :type Float%20%28single-precision%29))
  (Transformation|AddActorLocalRotation "0,1.000000, 0" false false)
  (bind _newtrack_0 (Timeline|Bob Play)
    (:Update
      (Transformation|AddActorLocalOffset _newtrack_0 false false))))

(fn ConstructionScript)